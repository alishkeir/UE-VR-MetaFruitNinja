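; BP_Chunks is a short-lived debris actor made of several static mesh chunks that burst apart when spawned.
; Its construction script applies a main and a chunk material to each mesh under Scene and scales SceneScale uniformly by a Scale variable.
; On BeginPlay it applies a small constant radial impulse to the chunks from the actor's location, then destroys itself after a brief delay.
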(event EventBeginPlay
  (Physics|AddRadialImpulse (Variables|Default|GetSM_Chunk4) (Transformation|GetActorLocation) 1e+01 3.0 "RIF_Constant" false)
  (Utilities|FlowControl|Delay 1.5)
  (Actor|DestroyActor))

(fn ConstructionScript
  (Utilities|FlowControl|Sequence
    (:then_0
      (for _array_element (Components|GetChildrenComponents (Variables|Default|GetScene) false)
        (bind _asstatic_mesh_component (Utilities|Casting|CastToStaticMeshComponent _array_element))
        (Rendering|Material|SetMaterial _asstatic_mesh_component 0 (Variables|Default|GetMainMaterial))
        (Rendering|Material|SetMaterial _asstatic_mesh_component 1 (Variables|Default|GetChunkMaterial))))
    (:then_1
      (Transformation|SetWorldScale3D (Variables|Default|GetsceneScale) (* "1.000000,1.000000,1.000000" (Variables|Default|GetScale))))))