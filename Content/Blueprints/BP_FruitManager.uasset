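; BP_FruitManager spawns random fruit for the player to hit and clears away any that are missed.
; After a short delay at BeginPlay, a self-repeating loop spawns one of five fruit classes at a random Y/Z offset around SpawnZone, using Start's rotation.
; Random wait times are divided by SpawnRatio to scale the spawn rate.
; Fruit overlapping the Box counts as failed, printing a message before being destroyed.
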(event OnComponentBeginOverlap(Box)
  (params (OverlappedComponent :type Primitive%20Component%20Object%20Reference) (OtherActor :type Actor%20Object%20Reference) (OtherComp :type Primitive%20Component%20Object%20Reference) (OtherBodyIndex :type Integer) (bFromSweep :type Boolean) (SweepResult :type Hit%20Result%20Structure%20%28by%20ref%29))
  (bind _as_bp_fruit (Utilities|Casting|CastTo_BP_Fruit OtherActor))
  (CallFunction|FruitFailed _as_bp_fruit))

(event Custom|SpawnFruit
  (bind _spawnzone (Variables|Default|GetSpawnZone))
  (bind _sphereradius (Variables|/Script/Engine.SphereComponent|GetSphereRadius _spawnzone))
  (Utilities|FlowControl|Sequence
    (:then_0
      (Game|SpawnActorfromClass (Utilities|Select :Index (Math|Random|RandomIntegerinRange 0 4) :Option%200 "/Game/Blueprints/BP_Apple.BP_Apple_C" :Option%201 "/Game/Blueprints/BP_Apple_Red.BP_Apple_Red_C" :Option%202 "/Game/Blueprints/BP_WaterMelon.BP_WaterMelon_C" :Option%203 "/Game/Blueprints/BP_Orange.BP_Orange_C" :Option%204 "/Game/Blueprints/BP_GrapeFruit.BP_GrapeFruit_C") (Math|Transform|MakeTransform (+ (Transformation|GetWorldLocation _spawnzone) (* (* "0.000000,1.000000,0.000000" _sphereradius) (Math|Random|RandomFloatinRange -1.0 1.0)) (* (* "0.000000,0.000000,1.000000" _sphereradius) (Math|Random|RandomFloatinRange -1.0 1.0))) (Transformation|GetWorldRotation (Variables|Default|GetStart))) "Undefined" 0 0))
    (:then_1
      (Utilities|FlowControl|Delay (/ (Math|Random|RandomFloatinRange 2.0 7.0) (Math|Float|Max(Float) (Variables|Default|GetSpawnRatio) 0.1)))
      (CallFunction|SpawnFruit))))

(event Custom|Init
  (CallFunction|SpawnFruit))

(event Custom|FruitFailed
  (params (Fruit :type BP%20Fruit%20Object%20Reference))
  (Utilities|FlowControl|Sequence
    (:then_0
      (Development|PrintString (Utilities|String|Append "We Failed To Hit: " (Utilities|GetDisplayName Fruit))))
    (:then_1
      (Actor|DestroyActor Fruit))))

(event EventBeginPlay
  (Utilities|FlowControl|Sequence
    (:then_0
      (Development|ExecuteConsoleCommand "start fps" 0))
    (:then_1
      (Utilities|FlowControl|Delay 2.0)
      (CallFunction|Init))))

(fn ConstructionScript)