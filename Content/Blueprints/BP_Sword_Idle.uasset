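; BP_Sword_Idle is a sword actor that bobs gently up and down in place, as an idle display effect.
; BeginPlay caches the actor's starting location.
; Tick offsets that location vertically by a sine of game time, so the motion stays centred on the spawn point and does not drift.
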(event EventBeginPlay
  (|CallParentFunction)
  (Variables|Default|SetDefaultLocation (Transformation|GetActorLocation)))

(event Collision|EventActorBeginOverlap
  (params (OtherActor :type Actor%20Object%20Reference)))

(event EventTick
  (params (DeltaSeconds :type Float%20%28single-precision%29))
  (Transformation|SetActorLocation (+ (Variables|Default|GetDefaultLocation) (* "0, 0,15.000000" (Math|Trig|Sin(Degrees) (* (Utilities|Time|GetGameTimeinSeconds) 1e+02)))) false false))

(fn ConstructionScript
  (|CallParentFunction))