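; BP_Fruit is a fruit actor that breaks apart the first time it is hit.
; On hit, a DoOnce disables collision on the collision mesh, hides the intact fruit mesh and shows a destructible sphere component in its place.
; It then activates that component and applies radius damage at the container's location to shatter it with an impulse.
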(event Custom|OnHit
  (bind _customsphere_dm (Variables|Default|GetCustomSphere_DM))
  (Utilities|FlowControl|DoOnce false
    (:Completed
      (Collision|SetCollisionEnabled (Variables|Default|GetCollisionMesh) "NoCollision")
      (Rendering|SetVisibility (Variables|Default|GetFruitMesh) false false)
      (Rendering|SetVisibility _customsphere_dm true false)
      (Components|Activation|Activate _customsphere_dm false)
      (Class|DestructibleComponent|ApplyRadiusDamage _customsphere_dm 5e+02 (Transformation|GetWorldLocation (Variables|Default|GetContainer)) 1e+01 5e+01 false))))

(fn ConstructionScript)