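; Base-style fruit actor that breaks apart once when OnHit fires, then destroys itself after a short delay.
; The hit disables collision, hides the mesh, and branches on ShouldUseApexDestruction.
; It either activates and radius-damages an Apex destructible sphere, or spawns BP_Chunks scaled to the collision sphere's radius.
; The construction script caches the mesh's main and chunk materials to pass to those chunks.
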(event Custom|OnHit
  (bind _customsphere_dm (Variables|Default|GetCustomSphere_DM))
  (Utilities|FlowControl|DoOnce false
    (:Completed
      (Utilities|FlowControl|Sequence
        (:then_0
          (Collision|SetCollisionEnabled (Variables|Default|GetCollisionMesh) "NoCollision")
          (Rendering|SetVisibility (Variables|Default|GetFruitMesh) false false)
          (if (Variables|Default|GetShouldUseApexDestruction)
            (Rendering|SetVisibility _customsphere_dm true false)
            (Components|Activation|Activate _customsphere_dm false)
            (Class|DestructibleComponent|ApplyRadiusDamage _customsphere_dm 5e+02 (Transformation|GetWorldLocation (Variables|Default|GetContainer)) 1e+01 3.0 false)
            (else
              (Game|SpawnActorfromClass "/Game/Asset/Blueprint/BP_Chunks.BP_Chunks_C" (Transformation|GetActorTransform) "Undefined" 0 (Variables|Default|GetMainMaterial) (Variables|Default|GetChunkMaterial) (/ (Variables|/Script/Engine.SphereComponent|GetSphereRadius (Variables|Default|GetCollisionMesh)) 21.0) 0))))
        (:then_1
          (Utilities|FlowControl|Delay 0.1)
          (Actor|DestroyActor))))))

(fn ConstructionScript
  (bind _fruitmesh (Variables|Default|GetFruitMesh))
  (Variables|Default|SetMainMaterial (Rendering|Material|GetMaterial _fruitmesh 0))
  (Variables|Default|SetChunkMaterial (Rendering|Material|GetMaterial _fruitmesh 1)))