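; Game mode for a VR fruit-slicing game with swords that runs the round lifecycle and tracks the total score.
; Shortly after play begins, it spawns an idle sword at every sword spawn point.
; Starting a game resets the score, starts the fruit manager and hides the pawn's score display.
; A failed fruit stops the round, shows the score, removes swords from the motion controllers and respawns idle swords after a delay.
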(event Custom|StartGame
  (if (not (Variables|Default|GetIsGameStarted))
    (Variables|Default|SetIsGameStarted true)
    (Variables|Default|SetTotalScore 0)
    (Utilities|FlowControl|Sequence
      (:then_0
        (bind _returnvalue (Actor|GetActorOfClass "/Game/Blueprints/_BP_FruitManager._BP_FruitManager_C"))
        (Utilities|IsValid _returnvalue
          (:Is%20Valid
            (Default|StartGame _returnvalue))))
      (:then_1
        (bind _returnvalue_2 (Actor|GetActorOfClass "/Game/Blueprints/BP_VRPawn.BP_VRPawn_C"))
        (Default|HideScore _returnvalue_2)))))

(event Custom|StopGame
  (Variables|Default|SetIsGameStarted false)
  (Utilities|FlowControl|Sequence
    (:then_0
      (bind _returnvalue (Actor|GetActorOfClass "/Game/Blueprints/BP_VRPawn.BP_VRPawn_C"))
      (Default|ShowScore _returnvalue (Variables|Default|GetTotalScore)))
    (:then_1
      (bind _returnvalue_2 (Actor|GetActorOfClass "/Game/Blueprints/_BP_FruitManager._BP_FruitManager_C"))
      (Utilities|IsValid _returnvalue_2
        (:Is%20Valid
          (Default|StopGame _returnvalue_2))))
    (:then_2
      (bind _outactors (Actor|GetAllActorsOfClass "/Game/VirtualRealityBP/Blueprints/BP_MotionController.BP_MotionController_C"))
      (for _array_element _outactors
        (Default|RemoveSword _array_element)))
    (:then_3
      (Utilities|FlowControl|Delay 3.0)
      (CallFunction|PrepareGame))))

(event Custom|AddScore
  (params (Score :type Integer))
  (Variables|Default|SetTotalScore (+ Score (Variables|Default|GetTotalScore))))

(event Custom|OnFruitFailed
  (CallFunction|StopGame))

(event Custom|PrepareGame
  (bind _outactors (Actor|GetAllActorsOfClass "/Game/Blueprints/BP_Sword_spawn.BP_Sword_Spawn_C"))
  (for _array_element _outactors
    (Game|SpawnActorfromClass "/Game/Blueprints/BP_Sword_Idle.BP_Sword_Idle_C" (Transformation|GetActorTransform _array_element) "Undefined" 0 0)))

(event EventBeginPlay
  (Utilities|FlowControl|Delay 1.0)
  (CallFunction|PrepareGame))

(fn ConstructionScript)